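; Interactable lamp that switches its point light on and off when the player interacts with it.
; Interact, gated by CanInteract, toggles the PointLight intensity between zero and a fixed brightness, using the intensity itself as the on/off state.
; On BeginPlay and after each toggle, it formats the widget prompt text with ON or OFF to show the action the next interaction performs.
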(event EventBeginPlay
  (CallFunction|SetWidgetPrompt (Utilities|Text|FormatText (Utilities|Text|MakeLiteralText (Variables|Default|GetPromptText)) (Utilities|String|SelectText "ON" "OFF" (== (Variables|/Script/Engine.LightComponentBase|GetIntensity (Variables|Default|GetPointLight)) 0.0)))))

(event EventInteract
  (bind _pointlight (Variables|Default|GetPointLight))
  (bind _intensity (Variables|/Script/Engine.LightComponentBase|GetIntensity _pointlight))
  (bind _returnvalue (== _intensity 0.0))
  (if (Variables|Default|GetCanInteract)
    (Rendering|Components|Light|SetIntensity (Variables|Default|GetPointLight) (Math|Float|SelectFloat 5e+03 0.0 _returnvalue))
    (CallFunction|SetWidgetPrompt (Utilities|Text|FormatText (Utilities|Text|MakeLiteralText (Variables|Default|GetPromptText)) (Utilities|String|SelectText "ON" "OFF" _returnvalue)))))

(fn ConstructionScript
  (|CallParentFunction))