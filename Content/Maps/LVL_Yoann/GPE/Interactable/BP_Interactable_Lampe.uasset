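; BP_Interactable_Lampe is an interactable lamp that toggles its point light on and off.
; On Interact, if allowed, it switches the light intensity between zero and a fixed brightness, using the current intensity as its state.
; At BeginPlay and after each toggle, it formats the prompt text with "On" or "Off" to name the next action and passes it to the prompt widget.
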(event EventBeginPlay
  (CallFunction|SetWidgetPrompt (Utilities|Text|FormatText (Variables|Default|GetPromptText) (Utilities|String|SelectText "On" "Off" (== (Variables|/Script/Engine.LightComponentBase|GetIntensity (Variables|Default|GetPointLight)) 0.0)))))

(event EventInteract
  (bind _pointlight (Variables|Default|GetPointLight))
  (bind _intensity (Variables|/Script/Engine.LightComponentBase|GetIntensity _pointlight))
  (bind _returnvalue (== _intensity 0.0))
  (if (Variables|Default|GetCaninteract)
    (Rendering|Components|Light|SetIntensity (Variables|Default|GetPointLight) (Math|Float|SelectFloat 5e+03 0.0 _returnvalue)) ; Switch ON
    (CallFunction|SetWidgetPrompt (Utilities|Text|FormatText (Variables|Default|GetPromptText) (Utilities|String|SelectText "On" "Off" _returnvalue)))))

(fn ConstructionScript
  (|CallParentFunction))